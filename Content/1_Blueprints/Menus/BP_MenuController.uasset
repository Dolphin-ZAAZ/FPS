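; Menu controller that handles input mode and back navigation for the game's menus.
; It swaps Enhanced Input mapping contexts between Default, Preview and UI, starting in UI on BeginPlay.
; It stores the active menu, and the secondary input action calls GoToPreviousMenu on it when it casts to BP_Menu.
; Its own GoToPreviousMenu function is an empty stub.
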(event Input|EnhancedActionEvents|EnhancedInputActionIA_Secondary
  (params (ActionValue :type Boolean) (ElapsedSeconds :type Float%20%28double-precision%29) (TriggeredSeconds :type Float%20%28double-precision%29) (InputAction :type Input%20Action%20Object%20Reference :default "/Game/2_Inputs/InputActions/Player/IA_Secondary.IA_Secondary"))
  (:Started
    (bind _asbp_menu (Utilities|Casting|CastToBP_Menu (Variables|Default|GetActiveMenu)))
    (Default|GotoPreviousMenu _asbp_menu)))

(event EventBeginPlay
  (CallFunction|SetInputMode "NewEnumerator2"))

(event EventTick
  (params (DeltaSeconds :type Float%20%28single-precision%29)))

(fn ConstructionScript)

(fn SetInputMode
  (params (InputState :type E_InputState%20Enum :default "NewEnumerator2"))
  (bind _returnvalue (Game|GetPlayerController 0))
  (bind _returnvalue_2 (PlayerController|LocalPlayerSubsystems|GetEnhancedInputLocalPlayerSubsystem _returnvalue))
  (Utilities|IsValid _returnvalue_2
    (:Is%20Valid
      (bind _output_get (Variables|Default|SetInputState InputState))
      (switch Utilities|FlowControl|Switch|SwitchonE_InputState _output_get
        (:NewEnumerator0
          (Input|RemoveMappingContext _returnvalue_2 "/Game/2_Inputs/IM_Preview.IM_Preview" "(bIgnoreAllPressedKeysUntilRelease=True,bForceImmediately=False,bNotifyUserSettings=False)")
          (Input|RemoveMappingContext _returnvalue_2 "/Game/2_Inputs/IM_UI.IM_UI" "(bIgnoreAllPressedKeysUntilRelease=True,bForceImmediately=False,bNotifyUserSettings=False)")
          (Input|AddMappingContext _returnvalue_2 "/Game/2_Inputs/IM_Default.IM_Default" 0 "(bIgnoreAllPressedKeysUntilRelease=True,bForceImmediately=False,bNotifyUserSettings=False)"))
        (:NewEnumerator1
          (Input|RemoveMappingContext _returnvalue_2 "/Game/2_Inputs/IM_Default.IM_Default" "(bIgnoreAllPressedKeysUntilRelease=True,bForceImmediately=False,bNotifyUserSettings=False)")
          (Input|RemoveMappingContext _returnvalue_2 "/Game/2_Inputs/IM_UI.IM_UI" "(bIgnoreAllPressedKeysUntilRelease=True,bForceImmediately=False,bNotifyUserSettings=False)")
          (Input|AddMappingContext _returnvalue_2 "/Game/2_Inputs/IM_Preview.IM_Preview" 0 "(bIgnoreAllPressedKeysUntilRelease=True,bForceImmediately=False,bNotifyUserSettings=False)"))
        (:NewEnumerator2
          (Input|RemoveMappingContext _returnvalue_2 "/Game/2_Inputs/IM_Preview.IM_Preview" "(bIgnoreAllPressedKeysUntilRelease=True,bForceImmediately=False,bNotifyUserSettings=False)")
          (Input|RemoveMappingContext _returnvalue_2 "/Game/2_Inputs/IM_Default.IM_Default" "(bIgnoreAllPressedKeysUntilRelease=True,bForceImmediately=False,bNotifyUserSettings=False)")
          (Input|AddMappingContext _returnvalue_2 "/Game/2_Inputs/IM_UI.IM_UI" 0 "(bIgnoreAllPressedKeysUntilRelease=True,bForceImmediately=False,bNotifyUserSettings=False)"))))))

(fn GotoPreviousMenu)

(fn SetActiveMenu
  (params (ActiveMenu :type Widget%20Object%20Reference))
  (Variables|Default|SetActiveMenu ActiveMenu))