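; Rifle item for the player inventory that handles hitscan firing, magazine ammo, reloading and aim-down-sights with an FOV change.
; Use is rate-limited by RoundsPerMinute, plays muzzle, sound and animation effects, and optionally spawns explosions at impact.
; Player raycast hits apply damage through I_Damageable, with a CritSpot component multiplier and instigator-only hitmarker feedback.
; Recoil follows sine-based yaw and pitch patterns indexed by shot count, which Tick resets after a delay.
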(event EventBeginPlay
  (Variables|Default|SetThisItem (Utilities|Struct|MakeST_Item "BP_Gun_C" "/Game/1_Blueprints/Player/InventorySystem/Items/Weapons/Icons/assault_rifle_icon_1_Sprite.assault_rifle_icon_1_Sprite" "Rifle" "This is a rifle." 2.0 1))
  (bind _output_get (Variables|Default|SetFireInterval (/ 1.0 (/ (Variables|Default|GetRoundsPerMinute) 6e+01))))
  (Variables|Default|SetFireIntervalTimer _output_get))

(event Collision|EventActorBeginOverlap
  (params (OtherActor :type Actor%20Object%20Reference)))

(event EventTick
  (params (DeltaSeconds :type Float%20%28single-precision%29))
  (Variables|Default|SetFireIntervalTimer (- (Variables|Default|GetFireIntervalTimer) DeltaSeconds))
  (if (<= (Variables|Recoil|GetRecoilResetCounter) 0.0)
    (CallFunction|ResetRecoilPatternProgress)
    (else
      (Variables|Recoil|SetRecoilResetCounter (- (Variables|Recoil|GetRecoilResetCounter) DeltaSeconds)))))

(fn ConstructionScript)

(fn Equip
  (params (OwningPlayer :type Boolean))
  (|CallParentFunction false)
  (CallFunction|ResetRecoilTimer))

(fn Use
  (params (PlayerRef :type BP%20Player%20Character%20Object%20Reference) (IsInstigator :type Boolean))
  (bind _hud (Variables|/Game/1_Blueprints/Player/BP_PlayerCharacter.BP_PlayerCharacter_C|GetHUD PlayerRef))
  (bind _damage (Variables|Default|GetDamage))
  (bind _camera (Variables|/Game/1_Blueprints/Player/BP_PlayerCharacter.BP_PlayerCharacter_C|GetCamera PlayerRef))
  (bind _returnvalue (Transformation|GetWorldLocation _camera))
  (|CallParentFunction PlayerRef IsInstigator)
  (if (not (Variables|Reloading|GetIsReloading))
    (if (< (Variables|Default|GetFireIntervalTimer) 0.0)
      (bind _isempty (CallFunction|CheckEmptyMag))
      (if (not _isempty)
        (bind _output_get (Variables|Reloading|SetRoundsIntMag (- (Variables|Reloading|GetRoundsIntMag) 1)))
        (if IsInstigator
          (Default|UpdateAmmo (Variables|/Game/1_Blueprints/Player/BP_PlayerCharacter.BP_PlayerCharacter_C|GetHUD PlayerRef) _output_get (Variables|Default|GetMagSize)))
        (CallFunction|AddRecoil PlayerRef)
        (Variables|Default|SetFireIntervalTimer (Variables|Default|GetFireInterval))
        (if (Variables|Default|GetIsEquipped)
          (bind _rayhit (Default|PlayerRaycast PlayerRef))
          (CallFunction|UseEffects _returnvalue)
          (if (Variables|Default|GetHasExplosiveBullets)
            (Game|SpawnActorfromClass "/Game/1_Blueprints/Player/BP_Explosion.BP_Explosion_C" (Math|Conversions|ToTransform(Vector) (.ImpactPoint (Collision|BreakHitResult _rayhit))) "Undefined" "MultiplyWithRoot" 0 0))
          (if (.bBlockingHit (Collision|BreakHitResult _rayhit))
            (bind _asi_damageable (Utilities|Casting|CastToI_Damageable (.HitActor (Collision|BreakHitResult _rayhit))))
            (bind _playerdamageable (Default|PlayerDamageable _asi_damageable))
            (if _playerdamageable
              (if (Utilities|Enum|Equal(Enum) (Utilities|GetObjectName (.HitComponent (Collision|BreakHitResult _rayhit))) "CritSpot")
                (Default|RemoveHealth _asi_damageable (* (Variables|Default|GetCritMultiplier) _damage) IsInstigator)
                (if IsInstigator
                  (Default|PlayHimarker _hud true)
                  (Audio|PlaySoundatLocation "/Game/4_Sounds/Impacts/Ting_Cue.Ting_Cue" _returnvalue "0, 0, 0" 1.0 1.0 0.0 0 0 0 0))
                (else
                  (Default|RemoveHealth _asi_damageable _damage IsInstigator)
                  (if IsInstigator
                    (Audio|PlaySoundatLocation "/Game/4_Sounds/Impacts/Bop_Cue.Bop_Cue" _returnvalue "0, 0, 0" 1.0 1.0 0.0 0 0 0 0)
                    (Default|PlayHimarker _hud false))))
              (Class|AISenseTouch|ReportTouchEvent (.HitActor (Collision|BreakHitResult _rayhit)) PlayerRef (.ImpactPoint (Collision|BreakHitResult _rayhit))))))))))

(fn Aim
  (params (PlayerRef :type BP%20Player%20Character%20Object%20Reference) (ShouldAim :type Boolean))
  (bind _hud (Variables|/Game/1_Blueprints/Player/BP_PlayerCharacter.BP_PlayerCharacter_C|GetHUD PlayerRef))
  (bind _camera (Variables|/Game/1_Blueprints/Player/BP_PlayerCharacter.BP_PlayerCharacter_C|GetCamera PlayerRef))
  (bind _aimfovchange (Variables|Default|GetAimFOVChange))
  (if ShouldAim
    (if (not (Variables|Reloading|GetIsReloading))
      (if (not (Variables|Default|GetIsAiming))
        (Transformation|SetRelativeTransform (Variables|Default|GetDefaultSceneRoot) (Variables|Default|GetAimTransform) false false)
        (Default|HideCrosshair _hud true)
        (Camera|SetFieldOfView _camera (- (Variables|/Script/Engine.CameraComponent|GetFieldOfView _camera) _aimfovchange))
        (Transformation|SetRelativeLocation (Variables|Default|GetMuzzleFlash) (Variables|/Script/Engine.SceneComponent|GetRelativeLocation (Variables|Default|GetBarrelPoint)) false false)
        (Variables|Default|SetIsAiming true)))
    (elif (Variables|Default|GetIsAiming)
      (CallFunction|Equip false)
      (Default|HideCrosshair _hud false)
      (Camera|SetFieldOfView _camera (+ (Variables|/Script/Engine.CameraComponent|GetFieldOfView _camera) _aimfovchange))
      (Transformation|SetRelativeLocation (Variables|Default|GetMuzzleFlash) (Variables|/Script/Engine.SceneComponent|GetRelativeLocation (Variables|Default|GetHipfireFlashPoint)) false false)
      (Variables|Default|SetIsAiming false))))

(fn CheckEmptyMag
  (return (<= (Variables|Reloading|GetRoundsIntMag) 0)))

(fn Reload
  (params (IsInstigator :type Boolean))
  (bind _magsize (Variables|Default|GetMagSize))
  (bind _output_get (Variables|Reloading|SetRoundsIntMag _magsize))
  (Variables|Reloading|SetIsReloading false)
  (return _output_get _magsize))

(fn CheckNotFullMag
  (return (< (Variables|Reloading|GetRoundsIntMag) (Variables|Default|GetMagSize))))

(fn AddRecoil
  (params (PlayerCharacter :type BP%20Player%20Character%20Object%20Reference))
  (CallFunction|ResetRecoilTimer)
  (Variables|Recoil|SetRecoilProgressCount (+ (Variables|Recoil|GetRecoilProgressCount) 1))
  (bind _amount (CallFunction|HorizontalRecoilFunction))
  (Pawn|Input|AddControllerYawInput PlayerCharacter _amount)
  (bind _amount_2 (CallFunction|VerticalRecoilFunction))
  (Pawn|Input|AddControllerPitchInput PlayerCharacter _amount_2))

(fn HorizontalRecoilFunction
  (return (+ (* (Variables|Recoil|GetHorizontalAmplitude) (Math|Trig|Sin(Degrees) (* (Variables|Recoil|GetHorizontalFrequency) (Variables|Recoil|GetRecoilProgressCount)))) (Variables|Recoil|GetHorizontalShift))))

(fn VerticalRecoilFunction
  (return (+ (* (Variables|Recoil|GetVetricalAmplitude) (Math|Trig|Sin(Degrees) (* (Variables|Recoil|GetVerticalFrequency) (Variables|Recoil|GetRecoilProgressCount)))) (Variables|Recoil|GetVerticalShift))))

(fn ResetRecoilPatternProgress
  (Variables|Recoil|SetRecoilProgressCount (Variables|Recoil|GetRecoilProgressOffset))
  (CallFunction|ResetRecoilTimer))

(fn ResetRecoilTimer
  (Variables|Recoil|SetRecoilResetCounter (Variables|Recoil|GetRecoilResetTime)))

(fn NewFunction
  (params (Location :type Vector))
  (Components|Activation|SetActive (Variables|Default|GetMuzzleFlash) true true)
  (Audio|PlaySoundatLocation "/Game/4_Sounds/Gunshots/Full-Auto_Cue.Full-Auto_Cue" Location "0, 0, 0" 1.0 1.0 0.0 0 0 0 0)
  (Components|Animation|PlayAnimation (Variables|Default|GetRifle_Assault_West_Rig) "/Game/6_Animation/AS_RecoilAnimation.AS_RecoilAnimation" false))

(fn UseEffects
  (params (Location :type Vector :default "0, 0, 0"))
  (|CallParentFunction Location)
  (if (not (Variables|Reloading|GetIsReloading))
    (Components|Activation|SetActive (Variables|Default|GetMuzzleFlash) true true)
    (Audio|PlaySoundatLocation "/Game/4_Sounds/Gunshots/Full-Auto_Cue.Full-Auto_Cue" Location "0, 0, 0" 1.0 1.0 0.0 0 0 0 0)
    (Components|Animation|PlayAnimation (Variables|Default|GetRifle_Assault_West_Rig) "/Game/6_Animation/AS_RecoilAnimation.AS_RecoilAnimation" false)))