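; BP_EnemyWaveHandler starts enemy waves on player input and tracks how many enemies remain.
; On play it caches the player and all spawners; StartWave sets the in-progress flag if BP_PathChecker reports a viable path.
; The input event then waits a countdown, spawns a batch at a random spawner and updates the remaining count, even when StartWave refuses.
; EndWave is an empty stub, so the flag is never cleared here.
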(event Input|EnhancedActionEvents|EnhancedInputActionIA_StartWave
  (params (ActionValue :type Boolean) (ElapsedSeconds :type Float%20%28double-precision%29) (TriggeredSeconds :type Float%20%28double-precision%29) (InputAction :type Input%20Action%20Object%20Reference :default "/Game/Inputs/InputActions/Level/IA_StartWave.IA_StartWave"))
  (bind _spawners (Variables|Default|GetSpawners))
  (bind _enemyspawneramount (Variables|Default|GetEnemySpawnerAmount))
  (CallFunction|StartWave)
  (Utilities|FlowControl|Delay (Variables|Default|GetEnemySpawnerCountdown))
  (Default|SpawnEnemies (Utilities|Array|Get(acopy) _spawners (- (Math|Random|RandomIntegerinRange 1 (Utilities|Array|Length _spawners)) 1)) _enemyspawneramount)
  (Variables|Default|SetEnemiesRemaining (- (Variables|Default|GetEnemyWaveCount) _enemyspawneramount)))

(event EventBeginPlay
  (Utilities|FlowControl|Sequence
    (:then_0
      (bind _outactors (Actor|GetAllActorsOfClass "/Game/Blueprints/Player/BP_PlayerCharacter.BP_PlayerCharacter_C"))
      (Variables|Default|SetPlayerRef (Utilities|Array|Get(acopy) _outactors))
      (bind _outactors_2 (Actor|GetAllActorsOfClass "/Game/Blueprints/BP_Spawner.BP_Spawner_C"))
      (Variables|Default|SetSpawners _outactors_2))
    (:then_1
      (Variables|Default|SetEnemiesRemaining (Variables|Default|GetEnemyWaveCount)))))

(fn StartWave
  (bind _returnvalue (Actor|GetActorOfClass "/Game/Blueprints/BP_PathChecker.BP_PathChecker_C"))
  (bind _returnvalue_2 (Default|GetPathViability _returnvalue))
  (if _returnvalue_2
    (if (Variables|Default|GetWaveInProgress)
      (Development|PrintString "Wave already in progress.")
      (else
        (Variables|Default|SetWaveInProgress true)))
    (else
      (Development|PrintString "No Viable Path, cannot start wave"))))

(fn EndWave)