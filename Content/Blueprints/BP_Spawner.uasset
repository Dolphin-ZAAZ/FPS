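; BP_Spawner is a spawner actor that creates zombie enemies around its own location.
; SpawnEnemies loops over the requested count, spawning a BP_EnemyZombie each time at a fixed world height.
; X and Y each take a component of a separate random unit vector scaled by SpawnRadius, plus a constant positive offset that shifts the spawn area off-centre.
; BeginPlay is empty, and nothing in the file calls SpawnEnemies.
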(event EventBeginPlay)

(fn ConstructionScript)

(fn SpawnEnemies
  (params (EnemyAmount :type Integer))
  (bind _returnvalue (Math|Random|RandomUnitVector))
  (bind _returnvalue_2 (Transformation|GetActorLocation))
  (bind _spawnradius (Variables|Default|GetSpawnRadius))
  (for _index (range 1 EnemyAmount)
    (Game|SpawnActorfromClass "/Game/Blueprints/Enemy/Zombie/BP_EnemyZombie.BP_EnemyZombie_C" (Math|Transform|MakeTransform (Math|Vector|MakeVector (+ (+ (* (.x _returnvalue) _spawnradius) 1e+02) (.x _returnvalue_2)) (+ (+ (* (.y _returnvalue) _spawnradius) 1e+02) (.y _returnvalue_2)) 1.5e+02) "0, 0, 0" "1.000000,1.000000,1.000000") "Undefined" "MultiplyWithRoot" 0 0)))