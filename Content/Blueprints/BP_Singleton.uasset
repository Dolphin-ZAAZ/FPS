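; BP_Singleton holds shared game state for player death and menu locking, exposed through getter and setter functions.
; RespawnPlayer looks up BP_PlayerCharacter by class and, if the player is flagged dead, calls Respawn on its C_PlayerVitals component and clears the flag.
; SetMenuLocked, as written, calls itself instead of assigning MenuLocked, and the Init event is empty.
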(event EventInit)

(fn GetPlayerIsDead
  (return (Variables|Default|GetPlayerIsDead)))

(fn SetPlayerIsDead
  (params (PlayerIsDead :type Boolean))
  (Variables|Default|SetPlayerIsDead PlayerIsDead))

(fn RespawnPlayer
  (bind _returnvalue (Actor|GetActorOfClass "/Game/Blueprints/BP_PlayerCharacter.BP_PlayerCharacter_C"))
  (bind _output_get (Variables|Default|SetPlayer _returnvalue))
  (if (Variables|Default|GetPlayerIsDead)
    (Default|Respawn (Actor|GetComponentbyClass _output_get "/Game/Blueprints/C_PlayerVitals.C_PlayerVitals_C"))
    (Variables|Default|SetPlayerIsDead false)))

(fn GetMenuLocked
  (return (Variables|Default|GetMenuLocked)))

(fn SetMenuLocked
  (params (LockMenu :type Boolean))
  (CallFunction|SetMenuLocked LockMenu))