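; Player inventory component that picks up items, stacks them by name and handles ten hotbar slots.
; Interact raycasts for a BP_ItemBase, adds and stores it, then updates the inventory UI, which supplies the hotbar contents pushed to the HUD.
; Hotbar inputs check class defaults, then either spawn equipables attached to the camera, replacing the held item, or spawn, use and destroy usables.
; Empty slots unequip; RemoveInventoryItem is an unimplemented stub.
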(event Input|EnhancedActionEvents|EnhancedInputActionIA_Interact
  (params (ActionValue :type Boolean) (ElapsedSeconds :type Float%20%28double-precision%29) (TriggeredSeconds :type Float%20%28double-precision%29) (InputAction :type Input%20Action%20Object%20Reference :default "/Game/Inputs/InputActions/Player/IA_Interact.IA_Interact"))
  (bind _rayhit (Default|PlayerRaycast (Variables|Default|GetPlayerRef)))
  (bind _asbp_item_base (Utilities|Casting|CastToBP_ItemBase (.hitactor _rayhit)))
  (CallFunction|AddInventoryItem (Variables|/Game/Blueprints/Items/BP_ItemBase.BP_ItemBase_C|GetThisItem _asbp_item_base))
  (Default|Store _asbp_item_base))

(event Input|EnhancedActionEvents|EnhancedInputActionIA_Hotbar1
  (params (ActionValue :type Boolean) (ElapsedSeconds :type Float%20%28double-precision%29) (TriggeredSeconds :type Float%20%28double-precision%29) (InputAction :type Input%20Action%20Object%20Reference :default "/Game/Inputs/InputActions/Inventory/IA_Hotbar1.IA_Hotbar1"))
  (CallFunction|EquipHotbarItem))

(event Input|EnhancedActionEvents|EnhancedInputActionIA_Hotbar10
  (params (ActionValue :type Boolean) (ElapsedSeconds :type Float%20%28double-precision%29) (TriggeredSeconds :type Float%20%28double-precision%29) (InputAction :type Input%20Action%20Object%20Reference :default "/Game/Inputs/InputActions/Inventory/IA_Hotbar10.IA_Hotbar10"))
  (CallFunction|EquipHotbarItem 9))

(event Input|EnhancedActionEvents|EnhancedInputActionIA_Hotbar2
  (params (ActionValue :type Boolean) (ElapsedSeconds :type Float%20%28double-precision%29) (TriggeredSeconds :type Float%20%28double-precision%29) (InputAction :type Input%20Action%20Object%20Reference :default "/Game/Inputs/InputActions/Inventory/IA_Hotbar2.IA_Hotbar2"))
  (CallFunction|EquipHotbarItem 1))

(event Input|EnhancedActionEvents|EnhancedInputActionIA_Hotbar3
  (params (ActionValue :type Boolean) (ElapsedSeconds :type Float%20%28double-precision%29) (TriggeredSeconds :type Float%20%28double-precision%29) (InputAction :type Input%20Action%20Object%20Reference :default "/Game/Inputs/InputActions/Inventory/IA_Hotbar3.IA_Hotbar3"))
  (CallFunction|EquipHotbarItem 2))

(event Input|EnhancedActionEvents|EnhancedInputActionIA_Hotbar4
  (params (ActionValue :type Boolean) (ElapsedSeconds :type Float%20%28double-precision%29) (TriggeredSeconds :type Float%20%28double-precision%29) (InputAction :type Input%20Action%20Object%20Reference :default "/Game/Inputs/InputActions/Inventory/IA_Hotbar4.IA_Hotbar4"))
  (CallFunction|EquipHotbarItem 3))

(event Input|EnhancedActionEvents|EnhancedInputActionIA_Hotbar5
  (params (ActionValue :type Boolean) (ElapsedSeconds :type Float%20%28double-precision%29) (TriggeredSeconds :type Float%20%28double-precision%29) (InputAction :type Input%20Action%20Object%20Reference :default "/Game/Inputs/InputActions/Inventory/IA_Hotbar5.IA_Hotbar5"))
  (CallFunction|EquipHotbarItem 4))

(event Input|EnhancedActionEvents|EnhancedInputActionIA_Hotbar6
  (params (ActionValue :type Boolean) (ElapsedSeconds :type Float%20%28double-precision%29) (TriggeredSeconds :type Float%20%28double-precision%29) (InputAction :type Input%20Action%20Object%20Reference :default "/Game/Inputs/InputActions/Inventory/IA_Hotbar6.IA_Hotbar6"))
  (CallFunction|EquipHotbarItem 5))

(event Input|EnhancedActionEvents|EnhancedInputActionIA_Hotbar7
  (params (ActionValue :type Boolean) (ElapsedSeconds :type Float%20%28double-precision%29) (TriggeredSeconds :type Float%20%28double-precision%29) (InputAction :type Input%20Action%20Object%20Reference :default "/Game/Inputs/InputActions/Inventory/IA_Hotbar7.IA_Hotbar7"))
  (CallFunction|EquipHotbarItem 6))

(event Input|EnhancedActionEvents|EnhancedInputActionIA_Hotbar8
  (params (ActionValue :type Boolean) (ElapsedSeconds :type Float%20%28double-precision%29) (TriggeredSeconds :type Float%20%28double-precision%29) (InputAction :type Input%20Action%20Object%20Reference :default "/Game/Inputs/InputActions/Inventory/IA_Hotbar8.IA_Hotbar8"))
  (CallFunction|EquipHotbarItem 7))

(event Input|EnhancedActionEvents|EnhancedInputActionIA_Hotbar9
  (params (ActionValue :type Boolean) (ElapsedSeconds :type Float%20%28double-precision%29) (TriggeredSeconds :type Float%20%28double-precision%29) (InputAction :type Input%20Action%20Object%20Reference :default "/Game/Inputs/InputActions/Inventory/IA_Hotbar9.IA_Hotbar9"))
  (CallFunction|EquipHotbarItem 8))

(event EventBeginPlay
  (bind _returnvalue (Components|GetOwner))
  (if (Pawn|IsLocallyControlled (Variables|/Script/Engine.Actor|GetInstigator _returnvalue))
    (bind _asbp_player_character (Utilities|Casting|CastToBP_PlayerCharacter _returnvalue))
    (bind _output_get (Variables|Default|SetPlayerRef _asbp_player_character))
    (Variables|Default|SetInventoryUIRef (Variables|/Game/Blueprints/Player/C_InventoryUIController.C_InventoryUIController_C|GetInventoryUI (Variables|/Game/Blueprints/Player/BP_PlayerCharacter.BP_PlayerCharacter_C|GetC_InventoryUIController _output_get)))))

(fn AddInventoryItem
  (params (Item :type ST%20Item%20Structure))
  (bind _inventoryuiref (Variables|Default|GetInventoryUIRef))
  (LocalVariables|SetQueryItem Item)
  (if (Utilities|Array|ContainsItem (Variables|Default|GetUniqueItems) (.name (LocalVariables|GetQueryItem)))
    (bind (_array_element _array_index) (Utilities|Array|ForEachLoopwithBreak (Variables|Default|GetInventoryItems) :!label _label)
      (:LoopBody
        (if (Utilities|Enum|Equal(Enum) (.name (.item _array_element)) (.name (LocalVariables|GetQueryItem)))
          (bind _output_get (LocalVariables|SetExistingItemIndex _array_index))
          (Utilities|Array|SetArrayElem (Variables|Default|GetInventoryItems) _output_get (Utilities|Struct|MakeST_InventoryItem (LocalVariables|GetQueryItem) (+ (.stackcount _array_element) 1) false 0))
          (goto _label Break)))
      (:Completed
        (Default|UpdateExistingSlot _inventoryuiref (Utilities|Array|Get(acopy) (Variables|Default|GetInventoryItems) (LocalVariables|GetExistingItemIndex)))
        (CallFunction|UpdateHotbarItems :!label _label_2)))
    (else
      (Utilities|Array|Add (Variables|Default|GetUniqueItems) (.name (LocalVariables|GetQueryItem)))
      (bind _returnvalue (Utilities|Array|Add (Variables|Default|GetInventoryItems) (Utilities|Struct|MakeST_InventoryItem (LocalVariables|GetQueryItem) 1 false 0)))
      (Default|AddtoEmptySlot _inventoryuiref (Utilities|Array|Get(acopy) (Variables|Default|GetInventoryItems) _returnvalue))
      (goto _label_2))))

(fn RemoveInventoryItem)

(fn ReadInventoryItems
  (return (Variables|Default|GetInventoryItems)))

(fn UpdateHotbarItems
  (bind _items (Default|ReadHotbarItems (Variables|Default|GetInventoryUIRef)))
  (bind _output_get (Variables|Default|SetHotbarItems _items))
  (Default|UpdateHotbar (Variables|/Game/Blueprints/Player/BP_PlayerCharacter.BP_PlayerCharacter_C|GetHUD (Variables|Default|GetPlayerRef)) _output_get))

(fn EquipHotbarItem
  (params (HotbarPosition :type Integer))
  (bind _hotbaritems (Variables|Default|GetHotbarItems))
  (bind _output (Utilities|Array|Get(acopy) _hotbaritems HotbarPosition))
  (bind _itemobject (Utilities|Struct|BreakST_Item (.item _output)))
  (if (> (Utilities|Array|Length _hotbaritems) 0)
    (if (Utilities|IsValidClass _itemobject)
      (if (not (== (Utilities|GetClass (Variables|Default|GetEquippedItem)) _itemobject))
        (bind _asbp_item_base (Utilities|Casting|CastToBP_ItemBaseClass _itemobject))
        (if (.IsEquipable (Utilities|GetClassDefaults _asbp_item_base))
          (if (Utilities|IsValidClass (Utilities|GetClass (Variables|Default|GetEquippedItem)))
            (Actor|DestroyActor (Variables|Default|GetEquippedItem)))
          (bind _returnvalue (Game|SpawnActorfromClass _itemobject (.EquipTransform (Utilities|GetClassDefaults _asbp_item_base)) "AlwaysSpawn" "MultiplyWithRoot" 0 0))
          (Transformation|AttachComponentToComponent _returnvalue (Variables|/Game/Blueprints/Player/BP_PlayerCharacter.BP_PlayerCharacter_C|GetCamera (Variables|Default|GetPlayerRef)) "None" "SnapToTarget" "SnapToTarget" "KeepRelative" true)
          (Default|Equip _returnvalue)
          (Variables|Default|SetEquippedItem _returnvalue)
          (elif (.IsUsable (Utilities|GetClassDefaults _asbp_item_base))
            (bind _returnvalue_2 (Game|SpawnActorfromClass _asbp_item_base (Math|Transform|MakeTransform "0, 0, 0" "0, 0, 0" "1.000000,1.000000,1.000000") "AlwaysSpawn" "MultiplyWithRoot" 0 0))
            (Default|Use _returnvalue_2)
            (Actor|DestroyActor _returnvalue_2))))
      (elif (Utilities|IsValid (Variables|Default|GetEquippedItem))
        (Actor|DestroyActor (Variables|Default|GetEquippedItem))
        (Variables|Default|SetEquippedItem 0)))))