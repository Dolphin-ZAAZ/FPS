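; BP_PhysicsBlock is a block that joins itself to neighboring blocks with breakable physics constraints.
; On BeginPlay it line-traces along six axes and adds a runtime constraint to each adjacent BP_PhysicsBlock found.
; Joints get tight angular limits and break above a scaled AngularThreshold.
; It then calls RefreshJoints on neighbors, which re-trace from cached axis endpoints and add joints when their joint count is below the trace count.
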(event EventBeginPlay
  (CallFunction|CreateInitialJoints))

(fn ConstructionScript)

(fn CreateInitialJoints
  (bind _staticmeshcomponent (Variables|Debug|GetStaticMeshComponent))
  (bind _returnvalue (Transformation|GetWorldLocation _staticmeshcomponent))
  (Utilities|Array|Add (Variables|Default|GetCube%20Axis) (+ _returnvalue "75.000000,0.000000,0.000000"))
  (Utilities|Array|Add (Variables|Default|GetCube%20Axis) (+ _returnvalue "0.000000,75.000000,0.000000"))
  (Utilities|Array|Add (Variables|Default|GetCube%20Axis) (+ _returnvalue "0.000000,0.000000,75.000000"))
  (Utilities|Array|Add (Variables|Default|GetCube%20Axis) (+ _returnvalue "-75.000000,0.000000,0.000000"))
  (Utilities|Array|Add (Variables|Default|GetCube%20Axis) (+ _returnvalue "0.000000,-75.000000,0.000000"))
  (Utilities|Array|Add (Variables|Default|GetCube%20Axis) (+ _returnvalue "0.000000,0.000000,-75.000000"))
  (for _array_element (Variables|Default|GetCube%20Axis)
    (bind _outhit (Collision|LineTraceForObjects (Transformation|GetWorldLocation (Variables|Debug|GetStaticMeshComponent)) _array_element (Variables|Default|GetObject%20Types) false 0 "None"))
    (Utilities|Array|Add (Variables|Default|GetAdjacentObjects) (.hitactor _outhit)))
  (for _array_element_2 (Variables|Default|GetAdjacentObjects)
    (bind _asbp_physics_block (Utilities|Casting|CastToBP_PhysicsBlock _array_element_2))
    (bind _returnvalue_2 (AddComponent|AddPhysicsConstraintComponent false))
    (Utilities|Array|Add (Variables|Default|GetJoints) _returnvalue_2)
    (Class|PhysicsConstraintComponent|SetConstrainedComponents _returnvalue_2 (Variables|Debug|GetStaticMeshComponent) "None" (Variables|/Script/Engine.StaticMeshActor|GetStaticMeshComponent _asbp_physics_block) "None"))
  (for _array_element_3 (Variables|Default|GetJoints)
    (bind _returnvalue_3 (Class|PhysicsConstraintComponent|GetConstraint _array_element_3))
    (Class|ConstraintInstanceBlueprintLibrary|SetAngularBreakable _returnvalue_3 true (* (Variables|Default|GetAngularThreshold) 1e+09))
    (Class|ConstraintInstanceBlueprintLibrary|SetAngularLimits _returnvalue_3 "ACM_Limited" 0.1 "ACM_Limited" 0.1 "ACM_Limited" 0.1))
  (for _array_element_4 (Variables|Default|GetAdjacentObjects)
    (bind _asbp_physics_block_2 (Utilities|Casting|CastToBP_PhysicsBlock _array_element_4))
    (CallFunction|RefreshJoints _asbp_physics_block_2)))

(fn RefreshJoints
  (Utilities|Array|Clear (Variables|Default|GetAdjacentObjects))
  (for _array_element (Variables|Default|GetCube%20Axis)
    (bind _outhit (Collision|LineTraceForObjects (Transformation|GetWorldLocation (Variables|Debug|GetStaticMeshComponent)) _array_element (Variables|Default|GetObject%20Types) false 0 "None"))
    (Utilities|Array|Add (Variables|Default|GetAdjacentObjects) (.hitactor _outhit)))
  (if (< (Utilities|Array|Length (Variables|Default|GetJoints)) (Utilities|Array|Length (Variables|Default|GetAdjacentObjects)))
    (for _array_element_2 (Variables|Default|GetAdjacentObjects)
      (bind _asbp_physics_block (Utilities|Casting|CastToBP_PhysicsBlock _array_element_2))
      (bind _array_element_3 (Utilities|Array|ForEachLoopwithBreak (Variables|Default|GetJoints) :!label _label)
        (:LoopBody
          (bind _outcomponent2 (Class|PhysicsConstraintComponent|GetConstrainedComponents _array_element_3))
          (if (== _outcomponent2 (Variables|/Script/Engine.StaticMeshActor|GetStaticMeshComponent _asbp_physics_block))
            (goto _label Break)
            (else
              (bind _returnvalue (AddComponent|AddPhysicsConstraintComponent false))
              (Class|PhysicsConstraintComponent|SetConstrainedComponents _returnvalue (Variables|Debug|GetStaticMeshComponent) "None" (Variables|/Script/Engine.StaticMeshActor|GetStaticMeshComponent _asbp_physics_block) "None")
              (Utilities|Array|Add (Variables|Default|GetJoints) _returnvalue))))))
    (for _array_element_4 (Variables|Default|GetJoints)
      (bind _returnvalue_2 (Class|PhysicsConstraintComponent|GetConstraint _array_element_4))
      (Class|ConstraintInstanceBlueprintLibrary|SetAngularBreakable _returnvalue_2 true (* (Variables|Default|GetAngularThreshold) 1e+09))
      (Class|ConstraintInstanceBlueprintLibrary|SetAngularLimits _returnvalue_2 "ACM_Limited" 0.1 "ACM_Limited" 0.1 "ACM_Limited" 0.1))))