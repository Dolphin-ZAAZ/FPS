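; BP_Gun is an equippable rifle item that the player fires, aims and reloads.
; Use gates shots by reload state, a Tick-driven fire-rate timer and magazine count, then plays recoil effects and updates the HUD.
; A player raycast damages I_Damageable targets with CritSpot multipliers, hitmarkers and touch-sense reporting, optionally spawning explosions at impact.
; Aim swaps the gun transform and muzzle-flash position, narrows FOV and hides the crosshair.
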(event EventBeginPlay
  (Variables|Default|SetThisItem (Utilities|Struct|MakeST_Item "BP_Gun_C" "/Game/Blueprints/Items/Weapons/Icons/assault_rifle_icon_1_Sprite.assault_rifle_icon_1_Sprite" "Rifle" "This is a rifle." 2.0 1))
  (bind _output_get (Variables|Default|SetFireInterval (/ 1.0 (/ (Variables|Default|GetRoundsPerMinute) 6e+01))))
  (Variables|Default|SetFireIntervalTimer _output_get))

(event Collision|EventActorBeginOverlap
  (params (OtherActor :type Actor%20Object%20Reference)))

(event EventTick
  (params (DeltaSeconds :type Float%20%28single-precision%29))
  (Variables|Default|SetFireIntervalTimer (- (Variables|Default|GetFireIntervalTimer) DeltaSeconds)))

(fn ConstructionScript)

(fn Equip
  (|CallParentFunction))

(fn Use
  (params (PlayerRef :type BP%20Player%20Character%20Object%20Reference))
  (bind _hud (Variables|/Game/Blueprints/Player/BP_PlayerCharacter.BP_PlayerCharacter_C|GetHUD PlayerRef))
  (bind _damage (Variables|Default|GetDamage))
  (bind _camera (Variables|/Game/Blueprints/Player/BP_PlayerCharacter.BP_PlayerCharacter_C|GetCamera PlayerRef))
  (bind _returnvalue (Transformation|GetWorldLocation _camera))
  (|CallParentFunction PlayerRef)
  (if (not (Variables|Default|GetIsReloading))
    (if (< (Variables|Default|GetFireIntervalTimer) 0.0)
      (bind _isempty (CallFunction|CheckEmptyMag))
      (if (not _isempty)
        (bind _output_get (Variables|Default|SetRoundsIntMag (- (Variables|Default|GetRoundsIntMag) 1)))
        (Default|UpdateAmmo (Variables|/Game/Blueprints/Player/BP_PlayerCharacter.BP_PlayerCharacter_C|GetHUD PlayerRef) _output_get (Variables|Default|GetMagSize))
        (Variables|Default|SetFireIntervalTimer (Variables|Default|GetFireInterval))
        (if (Variables|Default|GetIsEquipped)
          (bind _rayhit (Default|PlayerRaycast PlayerRef))
          (Components|Activation|SetActive (Variables|Default|GetMuzzleFlash) true true)
          (Audio|PlaySoundatLocation "/Game/Sounds/Gunshots/Full-Auto_Cue.Full-Auto_Cue" _returnvalue "0, 0, 0" 1.0 1.0 0.0 0 0 0 0)
          (Components|Animation|PlayAnimation (Variables|Default|GetRifle_Assault_West_Rig) "/Game/AS_RecoilAnimation.AS_RecoilAnimation" false)
          (if (Variables|Default|GetHasExplosiveBullets)
            (Game|SpawnActorfromClass "/Game/Blueprints/Player/BP_Explosion.BP_Explosion_C" (Math|Conversions|ToTransform(Vector) (.ImpactPoint (Collision|BreakHitResult _rayhit))) "Undefined" "MultiplyWithRoot" 0 0))
          (if (.bBlockingHit (Collision|BreakHitResult _rayhit))
            (bind _asi_damageable (Utilities|Casting|CastToI_Damageable (.HitActor (Collision|BreakHitResult _rayhit))))
            (Audio|PlaySoundatLocation "/Game/Sounds/Impacts/Bop_Cue.Bop_Cue" _returnvalue "0, 0, 0" 1.0 1.0 0.0 0 0 0 0)
            (bind _playerdamageable (Default|PlayerDamageable _asi_damageable))
            (if _playerdamageable
              (if (Utilities|Enum|Equal(Enum) (Utilities|GetObjectName (.HitComponent (Collision|BreakHitResult _rayhit))) "CritSpot")
                (Default|RemoveHealth _asi_damageable (* (Variables|Default|GetCritMultiplier) _damage))
                (Default|PlayHimarker _hud true)
                (Audio|PlaySoundatLocation "/Game/Sounds/Impacts/Ting_Cue.Ting_Cue" _returnvalue "0, 0, 0" 1.0 1.0 0.0 0 0 0 0)
                (else
                  (Default|RemoveHealth _asi_damageable _damage)
                  (Default|PlayHimarker _hud false)))
              (Class|AISenseTouch|ReportTouchEvent (.HitActor (Collision|BreakHitResult _rayhit)) PlayerRef (.ImpactPoint (Collision|BreakHitResult _rayhit))))))))))

(fn Aim
  (params (PlayerRef :type BP%20Player%20Character%20Object%20Reference) (ShouldAim :type Boolean))
  (bind _hud (Variables|/Game/Blueprints/Player/BP_PlayerCharacter.BP_PlayerCharacter_C|GetHUD PlayerRef))
  (bind _camera (Variables|/Game/Blueprints/Player/BP_PlayerCharacter.BP_PlayerCharacter_C|GetCamera PlayerRef))
  (bind _aimfovchange (Variables|Default|GetAimFOVChange))
  (if ShouldAim
    (if (not (Variables|Default|GetIsReloading))
      (if (not (Variables|Default|GetIsAiming))
        (Transformation|SetRelativeTransform (Variables|Default|GetDefaultSceneRoot) (Variables|Default|GetAimTransform) false false)
        (Default|HideCrosshair _hud true)
        (Camera|SetFieldOfView _camera (- (Variables|/Script/Engine.CameraComponent|GetFieldOfView _camera) _aimfovchange))
        (Transformation|SetRelativeLocation (Variables|Default|GetMuzzleFlash) (Variables|/Script/Engine.SceneComponent|GetRelativeLocation (Variables|Default|GetBarrelPoint)) false false)
        (Variables|Default|SetIsAiming true)))
    (elif (Variables|Default|GetIsAiming)
      (CallFunction|Equip)
      (Default|HideCrosshair _hud false)
      (Camera|SetFieldOfView _camera (+ (Variables|/Script/Engine.CameraComponent|GetFieldOfView _camera) _aimfovchange))
      (Transformation|SetRelativeLocation (Variables|Default|GetMuzzleFlash) (Variables|/Script/Engine.SceneComponent|GetRelativeLocation (Variables|Default|GetHipfireFlashPoint)) false false)
      (Variables|Default|SetIsAiming false))))

(fn CheckEmptyMag
  (return (<= (Variables|Default|GetRoundsIntMag) 0)))

(fn Reload
  (params (HUD :type UI%20HUD%20Object%20Reference))
  (bind _magsize (Variables|Default|GetMagSize))
  (bind _output_get (Variables|Default|SetRoundsIntMag _magsize))
  (Default|UpdateAmmo HUD _output_get _magsize)
  (Variables|Default|SetIsReloading false))

(fn CheckNotFullMag
  (return (< (Variables|Default|GetRoundsIntMag) (Variables|Default|GetMagSize))))