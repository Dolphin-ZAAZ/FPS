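; C_Jetpack is a component that gives its owning BP_PlayerCharacter an energy-limited jetpack on the jump input.
; The jump action drains energy from PlayerVitals, then applies upward force through CharacterMovement while energy remains and vertical speed is below MaxJetVelocity.
; A landed delegate assigned at BeginPlay refills energy with an oversized AddEnergy call.
; Energy is removed even when no force is applied.
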(event Custom|ResetEnergy
  (params (Hit :type Hit%20Result%20Structure%20%28by%20ref%29))
  (Default|AddEnergy (Variables|/Game/Blueprints/BP_PlayerCharacter.BP_PlayerCharacter_C|GetPlayerVitals (Variables|Default|GetPlayerRef)) 1e+06))

(event Input|EnhancedActionEvents|EnhancedInputActionIA_Jump
  (params (ActionValue :type Boolean) (ElapsedSeconds :type Float%20%28double-precision%29) (TriggeredSeconds :type Float%20%28double-precision%29) (InputAction :type Input%20Action%20Object%20Reference :default "/Game/Inputs/InputActions/IA_Jump.IA_Jump"))
  (bind _playerref (Variables|Default|GetPlayerRef))
  (bind _charactermovement (Variables|/Script/Engine.Character|GetCharacterMovement _playerref))
  (bind _playervitals (Variables|/Game/Blueprints/BP_PlayerCharacter.BP_PlayerCharacter_C|GetPlayerVitals _playerref))
  (Default|RemoveEnergy _playervitals)
  (if (< (.z (Variables|/Script/Engine.MovementComponent|GetVelocity _charactermovement)) (Variables|Default|GetMaxJetVelocity))
    (bind _energy (Default|GetVitals _playervitals))
    (if (> _energy 0.0)
      (Physics|AddForce _charactermovement (Math|Vector|MakeVector 0.0 0.0 (Variables|Default|GetJetForce))))))

(event EventBeginPlay
  (bind _asbp_player_character (Utilities|Casting|CastToBP_PlayerCharacter (Components|GetOwner)))
  (bind _output_get (Variables|Default|SetPlayerRef _asbp_player_character))
  (EventDispatchers|AssignLandedDelegate _output_get (delegate Custom|ResetEnergy)))