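; C_InventoryUIController controls the player's inventory screen, creating the UI_Inventory widget on BeginPlay and tracking its open and locked state.
; OpenInventory adds the widget to the viewport, while CloseInventory removes it, hides the mouse cursor and clears both state flags.
; LockInventory shows the mouse cursor and sets the locked flag, and getter functions expose both flags.
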(event EventBeginPlay
  (CallFunction|ConstructInventoryUI))

(fn OpenInventory
  (UserInterface|Viewport|AddtoViewport (Variables|Default|GetInventoryUI) 0)
  (Variables|Default|SetInventoryOpen true))

(fn CloseInventory
  (Widget|RemovefromParent (Variables|Default|GetInventoryUI))
  (Variables|/Script/Engine.PlayerController|SetbShowMouseCursor (Game|GetPlayerController (Variables|/Script/Engine.Pawn|GetPlayerState (Game|GetPlayerCharacter 0))) false)
  (Variables|Default|SetInventoryOpen false)
  (Variables|Default|SetInventoryLocked false))

(fn LockInventory
  (Variables|/Script/Engine.PlayerController|SetbShowMouseCursor (Game|GetPlayerController (Variables|/Script/Engine.Pawn|GetPlayerState (Game|GetPlayerCharacter 0))) true)
  (Variables|Default|SetInventoryLocked true))

(fn GetInventoryOpen
  (return (Variables|Default|GetInventoryOpen)))

(fn GetInventoryLocked
  (return (Variables|Default|GetInventoryLocked)))

(fn ConstructInventoryUI
  (bind _returnvalue (UserInterface|CreateWidget "/Game/Blueprints/UI/UI_Inventory.UI_Inventory_C" (Game|GetPlayerController 0)))
  (Variables|Default|SetInventoryUI _returnvalue))