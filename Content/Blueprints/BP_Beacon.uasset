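; BP_Beacon is a beacon Blueprint with Health, MaxHealth and IsDestroyed state.
; AddHealth sets Health to the passed amount, rather than the sum, when the sum is within MaxHealth, and to MaxHealth otherwise.
; RemoveHealth does nothing: its subtraction and destroyed-flag logic is disconnected from the entry.
; The event graph and construction script are empty.
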(event EventBeginPlay)

(event Collision|EventActorBeginOverlap
  (params (OtherActor :type Actor%20Object%20Reference)))

(event EventTick
  (params (DeltaSeconds :type Float%20%28single-precision%29)))

(fn ConstructionScript)

(fn RemoveHealth
  (params (HealthAmount :type Float%20%28double-precision%29)))

(fn AddHealth
  (params (HealthAmount :type Float%20%28double-precision%29))
  (if (<= (+ HealthAmount (Variables|Default|GetHealth)) (Variables|Default|GetMaxHealth))
    (Variables|Default|SetHealth HealthAmount)
    (else
      (Variables|Default|SetHealth (Variables|Default|GetMaxHealth)))))