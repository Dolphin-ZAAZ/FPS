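; Wave controller for an enemy-wave game that caches the player and all BP_Spawner actors at BeginPlay.
; StartWave sets WaveInProgress only if BP_PathChecker reports a viable path and no wave is running.
; During a wave, Tick feeds a gate that leads to a delayed spawn at a random spawner.
; The gate's Open and StartWave calls in the event graph are unconnected, and EndWave is empty.
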(event EventBeginPlay
  (Utilities|FlowControl|Sequence
    (:then_0
      (bind _outactors (Actor|GetAllActorsOfClass "/Game/Blueprints/Player/BP_PlayerCharacter.BP_PlayerCharacter_C"))
      (Variables|Default|SetPlayerRef (Utilities|Array|Get(acopy) _outactors))
      (bind _outactors_2 (Actor|GetAllActorsOfClass "/Game/Blueprints/BP_Spawner.BP_Spawner_C"))
      (for _array_element _outactors_2
        (Utilities|Array|Add (Variables|Default|GetSpawners) _array_element)))
    (:then_1
      (Variables|Default|SetEnemiesRemaining (Variables|Default|GetEnemyWaveCount)))))

(event EventTick
  (params (DeltaSeconds :type Float%20%28single-precision%29))
  (bind _spawners (Variables|Default|GetSpawners))
  (bind _enemyspawneramount (Variables|Default|GetEnemySpawnerAmount))
  (if (Variables|Default|GetWaveInProgress)
    (Utilities|FlowControl|Gate true :!label _label
      (:Exit
        (Utilities|FlowControl|Delay (Variables|Default|GetEnemySpawnerCountdown))
        (Default|SpawnEnemies (Utilities|Array|Get(acopy) _spawners (- (Math|Random|RandomIntegerinRange 1 (Utilities|Array|Length _spawners)) 1)) _enemyspawneramount)
        (Variables|Default|SetEnemiesRemaining (- (Variables|Default|GetEnemyWaveCount) _enemyspawneramount))))
    (else
      (goto _label Close))))

(fn ConstructionScript)

(fn StartWave
  (bind _returnvalue (Actor|GetActorOfClass "/Game/Blueprints/BP_PathChecker.BP_PathChecker_C"))
  (bind _returnvalue_2 (Default|GetPathViability _returnvalue))
  (if _returnvalue_2
    (if (Variables|Default|GetWaveInProgress)
      (Development|PrintString "Wave already in progress.")
      (else
        (Variables|Default|SetWaveInProgress true)))
    (else
      (Development|PrintString "No Viable Path, cannot start wave"))))

(fn EndWave)