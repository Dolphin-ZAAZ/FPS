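; BP_HeavyBullet is a physics-driven projectile that damages enemy shooters and the player character.
; On BeginPlay it launches its Sphere with a forward impulse scaled by BulletForce.
; On actor overlap it calls RemoveHealth on a BP_EnemyShooter, or otherwise deals fixed damage through the player's CPlayerVitals component.
; The bullet's graph has no destroy step after a hit.
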(event EventBeginPlay
  (Physics|AddImpulse (Variables|Default|GetSphere) (* (Math|Vector|GetForwardVector (Transformation|GetWorldRotation (Variables|Default|GetSphere))) (Variables|Default|GetBulletForce)) "None" false))

(event Collision|EventActorBeginOverlap
  (params (OtherActor :type Actor%20Object%20Reference))
  (bind _asbp_enemy_shooter (Utilities|Casting|CastToBP_EnemyShooter OtherActor)
    (:then
      (if (Utilities|IsValid _asbp_enemy_shooter)
        (Default|RemoveHealth _asbp_enemy_shooter)
        (else
          (Class|AutomationBlueprintFunctionLibrary|AddExpectedLogError "Expected Hit Object to be BP_Enemy"))))
    (:CastFailed
      (bind _asbp_player_character (Utilities|Casting|CastToBP_PlayerCharacter OtherActor))
      (if (Utilities|IsValid _asbp_player_character)
        (Default|RemoveHealth (Variables|/Game/Blueprints/Player/BP_PlayerCharacter.BP_PlayerCharacter_C|GetC_PlayerVitals _asbp_player_character) 1e+01)))))

(fn ConstructionScript)