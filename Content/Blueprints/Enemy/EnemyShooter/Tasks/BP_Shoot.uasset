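; Behavior tree task that makes an enemy shooter fire one heavy bullet.
; It skips firing when the global singleton game instance reports the player dead.
; Otherwise it spawns BP_HeavyBullet at the pawn's Gun-tagged component, aimed along that component's forward vector with random cone spread for inaccuracy.
; The task finishes successfully in both cases, but never finishes if the game instance cast fails.
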(event EventReceiveExecuteAI
  (params (OwnerController :type AI%20Controller%20Object%20Reference) (ControlledPawn :type Pawn%20Object%20Reference))
  (bind _returnvalue (Actor|GetComponentsbyTag ControlledPawn "/Script/Engine.SceneComponent" "Gun"))
  (bind _output (Utilities|Array|Get(acopy) _returnvalue))
  (bind _asbp_global_singleton (Utilities|Casting|CastToBP_GlobalSingleton (Game|GetGameInstance)))
  (bind _playerisdead (Default|GetPlayerIsDead _asbp_global_singleton))
  (if _playerisdead
    (AI|BehaviorTree|FinishExecute true)
    (else
      (Game|SpawnActorfromClass "/Game/Blueprints/Enemy/EnemyShooter/BP_HeavyBullet.BP_HeavyBullet_C" (Math|Transform|MakeTransform (Transformation|GetWorldLocation _output) (Math|Conversions|RotationFromXVector (Math|Random|RandomUnitVectorinConeinDegrees (Math|Vector|GetForwardVector _output) 5.0))) "Undefined" "MultiplyWithRoot" 0 0)
      (AI|BehaviorTree|FinishExecute true))))