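; Enemy AI controller that runs the BT_Enemy behavior tree and feeds it perception data through the Blackboard.
; On BeginPlay it starts the tree and seeds a GunAccuracy value.
; Each perception update stores the reported actor as Target, even when sight is lost.
; HasVision reflects whether the first currently sight-perceived actor is valid, with debug prints showing the result.
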(event OnTargetPerceptionUpdated(AIPerception)
  (params (Actor :type Actor%20Object%20Reference) (Stimulus :type AI%20Stimulus%20Structure))
  (bind _blackboard (Variables|Default|GetBlackboard))
  (AI|Components|Blackboard|SetValueasObject _blackboard (Utilities|Name|MakeLiteralName "Target") Actor)
  (if (Utilities|IsValid (Utilities|Array|Get(acopy) (Class|AIPerceptionComponent|GetCurrentlyPerceivedActors (Variables|Default|GetAIPerception) "/Script/AIModule.AISense_Sight")))
    (AI|Components|Blackboard|SetValueasBool _blackboard (Utilities|Name|MakeLiteralName "HasVision") true)
    (Development|PrintString "InSight")
    (else
      (AI|Components|Blackboard|SetValueasBool _blackboard (Utilities|Name|MakeLiteralName "HasVision") false)
      (Development|PrintString "Not InSight"))))

(event EventBeginPlay
  (AI|RunBehaviorTree "/Game/Blueprints/Enemy/BT_Enemy.BT_Enemy")
  (AI|Components|Blackboard|SetValueasFloat (Variables|Default|GetBlackboard) (Utilities|Name|MakeLiteralName "GunAccuracy") 1e+01))

(fn ConstructionScript)