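; Behavior tree task for the zombie enemy that deals a fixed amount of damage to its current blackboard Target.
; It casts the Target to the player character, removing health through its vitals component, or to a beacon, removing health directly.
; It fails for any other target type but reports success when the Target is invalid.
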(event EventReceiveExecuteAI
  (params (OwnerController :type AI%20Controller%20Object%20Reference) (ControlledPawn :type Pawn%20Object%20Reference))
  (bind _blackboardkeyselector (Utilities|Struct|MakeBlackboardKeySelector 0 "Target"))
  (bind _returnvalue (Class|BTFunctionLibrary|GetBlackboardValueasObject _blackboardkeyselector))
  (Utilities|IsValid _returnvalue
    (:Is%20Valid
      (bind _asbp_player_character (Utilities|Casting|CastToBP_PlayerCharacter _returnvalue)
        (:then
          (Default|RemoveHealth (Variables|/Game/Blueprints/Player/BP_PlayerCharacter.BP_PlayerCharacter_C|GetC_PlayerVitals _asbp_player_character) 1e+01)
          (AI|BehaviorTree|FinishExecute true))
        (:CastFailed
          (bind _asbp_beacon (Utilities|Casting|CastToBP_Beacon _returnvalue)
            (:then
              (Default|RemoveHealth _asbp_beacon 1e+01 false)
              (AI|BehaviorTree|FinishExecute true))
            (:CastFailed
              (AI|BehaviorTree|FinishExecute false))))))
    (:Is%20Not%20Valid
      (AI|BehaviorTree|FinishExecute true))))