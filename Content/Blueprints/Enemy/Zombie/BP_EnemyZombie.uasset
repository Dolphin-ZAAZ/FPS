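; BP_EnemyZombie is a zombie enemy actor that holds health and reports itself as damageable by the player.
; AddHealth caps healing at MaxHealth, while RemoveHealth subtracts damage and destroys the actor once health reaches zero or below.
; GetHealth returns current and maximum health, and PlayerDamageable always returns true.
; The file contains no movement, AI or attack logic, and BeginPlay and the construction script are empty.
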(event EventBeginPlay)

(event EventAddHealth
  (params (Health%20Amount :type Float%20%28double-precision%29))
  (if (<= (+ Health%20Amount (Variables|Default|GetHealth)) (Variables|Default|GetMaxHealth))
    (Variables|Default|SetHealth (+ Health%20Amount (Variables|Default|GetHealth)))
    (else
      (Variables|Default|SetHealth (Variables|Default|GetMaxHealth)))))

(event EventRemoveHealth
  (params (HealthAmount :type Float%20%28double-precision%29))
  (bind _output_get (Variables|Default|SetHealth (- (Variables|Default|GetHealth) HealthAmount)))
  (if (<= _output_get 0.0)
    (Actor|DestroyActor)))

(fn ConstructionScript)

(fn GetHealth
  (return (Variables|Default|GetHealth) (Variables|Default|GetMaxHealth)))

(fn PlayerDamageable
  (return true))