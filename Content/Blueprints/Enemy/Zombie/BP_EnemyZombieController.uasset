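; AI controller for the zombie enemy, which targets the nearest beacon by default and can switch to actors it senses.
; On possess it runs the zombie behavior tree, seeds blackboard attack values and sets the closest BP_Beacon as Target.
; While the player lives, sight of "Targetable" actors sets HasVision according to whether Target is empty, and touch perception retargets to the updated actor.
; The player's death event refocuses it on a beacon.
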(event OnTargetPerceptionUpdated(AIPerception)
  (params (Actor :type Actor%20Object%20Reference) (Stimulus :type AI%20Stimulus%20Structure))
  (bind _aiperception (Variables|Default|GetAIPerception))
  (bind _asbp_global_singleton (Utilities|Casting|CastToBP_GlobalSingleton (Game|GetGameInstance)))
  (bind _playerisdead (Default|GetPlayerIsDead _asbp_global_singleton))
  (if (not _playerisdead)
    (Utilities|FlowControl|Sequence
      (:then_0
        (for _array_element (Class|AIPerceptionComponent|GetCurrentlyPerceivedActors _aiperception "/Script/AIModule.AISense_Sight")
          (if (Actor|ActorHasTag _array_element "Targetable")
            (if (Actor|ActorHasTag _array_element "Targetable")
              (if (Utilities|IsValid (AI|Components|Blackboard|GetValueasObject (Variables|Default|GetBB) (Utilities|Name|MakeLiteralName "Target")))
                (AI|Components|Blackboard|SetValueasBool (Variables|Default|GetBB) (Utilities|Name|MakeLiteralName "HasVision") false)
                (else
                  (AI|Components|Blackboard|SetValueasBool (Variables|Default|GetBB) (Utilities|Name|MakeLiteralName "HasVision") true)))))))
      (:then_1
        (if (Utilities|IsValid (Utilities|Array|Get(acopy) (Class|AIPerceptionComponent|GetCurrentlyPerceivedActors _aiperception "/Script/AIModule.AISense_Touch")))
          (AI|Components|Blackboard|SetValueasObject (Variables|Default|GetBB) (Utilities|Name|MakeLiteralName "Target") Actor)
          (Development|PrintString "Hello"))))))

(event Custom|RefocusBeacon
  ;[1 1 1] Constructor
  (CallFunction|FocusBeacon))

(event EventPossess
  (params (PossessedPawn :type Pawn%20Object%20Reference))
  (bind _returnvalue (AI|GetAIController PossessedPawn))
  (AddComponent|AddBehaviorTreeComponent PossessedPawn)
  (AI|RunBehaviorTree _returnvalue "/Game/Blueprints/Enemy/Zombie/BT_EnemyZombie.BT_EnemyZombie")
  ;[1 1 1] Constructor
  (bind _blackboardcomponent (Class|AIController|UseBlackboard _returnvalue "/Game/Blueprints/Enemy/Zombie/BB_EnemyZombie.BB_EnemyZombie"))
  (bind _output_get (Variables|Default|SetBB _blackboardcomponent))
  (AI|Components|Blackboard|SetValueasFloat _output_get (Utilities|Name|MakeLiteralName "AttackDamage") 1e+01)
  (AI|Components|Blackboard|SetValueasObject _output_get (Utilities|Name|MakeLiteralName "SelfActor") PossessedPawn)
  (AI|Components|Blackboard|SetValueasFloat _output_get (Utilities|Name|MakeLiteralName "AttackRange") 2.5e+02)
  (CallFunction|FocusBeacon)
  (bind _asbp_player_character (Utilities|Casting|CastToBP_PlayerCharacter (Game|Player|GetPlayerPawn 0)))
  (EventDispatchers|BindEventtoPlayerDied (Variables|/Game/Blueprints/Player/BP_PlayerCharacter.BP_PlayerCharacter_C|GetPlayerVitals _asbp_player_character) (delegate Custom|RefocusBeacon)))

(fn ConstructionScript)

(fn FocusBeacon
  (bind _outactors (Actor|GetAllActorsOfClass "/Game/Blueprints/BP_Beacon.BP_Beacon_C"))
  (Variables|Default|SetClosestBeacon (Utilities|Array|Get(acopy) _outactors))
  (for _array_element _outactors
    (if (< (Math|Vector|Distance(Vector) (Transformation|GetActorLocation) (Transformation|GetActorLocation _array_element)) (Math|Vector|Distance(Vector) (Transformation|GetActorLocation) (Transformation|GetActorLocation (Variables|Default|GetClosestBeacon))))
      (bind _output_get (Variables|Default|SetClosestBeacon _array_element))
      (AI|Components|Blackboard|SetValueasObject (Variables|Default|GetBlackboard) (Utilities|Name|MakeLiteralName "Target") _output_get)
      (else
        (AI|Components|Blackboard|SetValueasObject (Variables|Default|GetBlackboard) (Utilities|Name|MakeLiteralName "Target") (Variables|Default|GetClosestBeacon))))))