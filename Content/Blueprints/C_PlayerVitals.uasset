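; C_PlayerVitals is a player component that tracks health and handles death and respawn.
; Health changes clamp to MaxHealth from the owner's PlayerStats, and reaching zero shows UI_DeathScreen with UI-only input, guarded by a dead flag in BP_Singleton.
; Respawn restores health, game input and the world-origin position, but leaves that flag set.
; Energy, hunger, thirst and their depletion functions are empty stubs.
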(event EventBeginPlay
  (bind _asbp_player_character (Utilities|Casting|CastToBP_PlayerCharacter (Components|GetOwner)))
  (Variables|Default|SetCurrentPlayer _asbp_player_character))

(fn RemoveHealth
  (params (HealthAmount :type Float%20%28double-precision%29))
  (bind _output_get (Variables|Default|SetHealth (- (Variables|Default|GetHealth) HealthAmount)))
  (if (<= _output_get 0.0)
    (CallFunction|KillPlayer)))

(fn AddHealth
  (params (HealthAmount :type Float%20%28double-precision%29))
  (bind _newparam (CallFunction|GetStats))
  (if (> (+ HealthAmount (Variables|Default|GetHealth)) (.maxhealth _newparam))
    (Variables|Default|SetHealth (.maxhealth _newparam))
    (else
      (Variables|Default|SetHealth (+ HealthAmount (Variables|Default|GetHealth))))))

(fn RemoveEnergy)

(fn AddEnergy)

(fn RemoveHunger)

(fn AddHunger)

(fn RemoveThirst)

(fn AddThirst)

(fn Dehydrated)

(fn Starving)

(fn Exhausted)

(fn KillPlayer
  (bind _returnvalue (Game|GetPlayerController 0))
  (bind _asbp_singleton (Utilities|Casting|CastToBP_Singleton (Game|GetGameInstance)))
  (bind _playerisdead (Default|GetPlayerIsDead _asbp_singleton))
  (if (not _playerisdead)
    (bind _returnvalue_2 (UserInterface|CreateWidget "/Game/Blueprints/UI/UI_DeathScreen.UI_DeathScreen_C" _returnvalue))
    (bind _output_get (Variables|Default|SetDeathScreen _returnvalue_2))
    (UserInterface|Viewport|AddtoViewport _output_get 0)
    (Variables|/Script/Engine.PlayerController|SetbShowMouseCursor _returnvalue true)
    (Input|SetInputModeUIOnly _returnvalue 0 "DoNotLock" false)
    (bind _asbp_singleton_2 (Utilities|Casting|CastToBP_Singleton (Game|GetGameInstance)))
    (Default|SetPlayerIsDead _asbp_singleton_2 true)))

(fn GetStats
  (bind _asbp_player_character (Utilities|Casting|CastToBP_PlayerCharacter (Components|GetOwner)))
  (return (Variables|/Game/Blueprints/C_PlayerStats.C_PlayerStats_C|GetStats (Variables|/Game/Blueprints/BP_PlayerCharacter.BP_PlayerCharacter_C|GetPlayerStats _asbp_player_character))))

(fn Respawn
  (bind _returnvalue (Game|GetPlayerController 0))
  (Widget|RemovefromParent (Variables|Default|GetDeathScreen))
  (Transformation|SetActorLocation (Components|GetOwner) "0, 0, 0" false false)
  (Input|SetInputModeGameOnly _returnvalue false)
  (Variables|/Script/Engine.PlayerController|SetbShowMouseCursor _returnvalue false)
  (bind _newparam (CallFunction|GetStats))
  (Variables|Default|SetHealth (.maxhealth _newparam)))

(fn GetVitals)