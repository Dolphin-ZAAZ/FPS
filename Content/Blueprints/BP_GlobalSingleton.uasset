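; BP_GlobalSingleton is a global state object tracking player death, game over and whether a wave is in progress.
; Init caches the BP_PlayerCharacter, and RespawnPlayer looks it up again, then calls Respawn on its C_PlayerVitals and clears the death flag if set.
; SetGameOver shows UI_GameOverScreen with the mouse cursor and UI-only input.
; StartWave and EndWave only toggle the wave flag.
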(event EventInit
  (bind _outactors (Actor|GetAllActorsOfClass "/Game/Blueprints/Player/BP_PlayerCharacter.BP_PlayerCharacter_C"))
  (Variables|Default|SetPlayer (Utilities|Array|Get(acopy) _outactors)))

(fn GetPlayerIsDead
  (return (Variables|Default|GetPlayerIsDead)))

(fn SetPlayerIsDead
  (params (PlayerIsDead :type Boolean))
  (Variables|Default|SetPlayerIsDead PlayerIsDead))

(fn RespawnPlayer
  (bind _returnvalue (Actor|GetActorOfClass "/Game/Blueprints/Player/BP_PlayerCharacter.BP_PlayerCharacter_C"))
  (bind _output_get (Variables|Default|SetPlayer _returnvalue))
  (if (Variables|Default|GetPlayerIsDead)
    (Default|Respawn (Actor|GetComponentbyClass _output_get "/Game/Blueprints/Player/C_PlayerVitals.C_PlayerVitals_C"))
    (Variables|Default|SetPlayerIsDead false)))

(fn SetGameOver
  (bind _returnvalue (Game|GetPlayerController 0))
  (Variables|Default|SetGameOver true)
  (bind _returnvalue_2 (UserInterface|CreateWidget "/Game/Blueprints/UI/UI_GameOverScreen.UI_GameOverScreen_C" _returnvalue))
  (UserInterface|Viewport|AddtoViewport _returnvalue_2 0)
  (Variables|/Script/Engine.PlayerController|SetbShowMouseCursor _returnvalue true)
  (Input|SetInputModeUIOnly _returnvalue 0 "DoNotLock" false))

(fn StartWave
  (Variables|Default|SetWaveInProgress true))

(fn EndWave
  (Variables|Default|SetWaveInProgress false))