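; Player component that fires ball projectiles from the camera on the primary input action.
; On BeginPlay it caches the owning BP_PlayerCharacter, whose camera transform and look direction place each BP_ProjectileBall spawn slightly ahead of the view.
; A Gate throttles firing by closing after each shot and reopening on input completion or through a fire-rate Delay branch driven by the input's elapsed time.
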(event Input|EnhancedActionEvents|EnhancedInputActionIA_Primary
  (params (ActionValue :type Boolean) (ElapsedSeconds :type Float%20%28double-precision%29) (TriggeredSeconds :type Float%20%28double-precision%29) (InputAction :type Input%20Action%20Object%20Reference :default "/Game/Inputs/InputActions/IA_Primary.IA_Primary"))
  (bind _balllauncherfirerate (Variables|Default|GetBallLauncherFireRate))
  (bind _playerref (Variables|Default|GetPlayerRef))
  (bind _camera (Variables|/Game/Blueprints/BP_PlayerCharacter.BP_PlayerCharacter_C|GetCamera _playerref))
  (bind _returnvalue (Transformation|GetWorldTransform _camera))
  ;[1 1 1] Ball Launcher
  (if (> (+ ElapsedSeconds _balllauncherfirerate) _balllauncherfirerate)
    (Utilities|FlowControl|Delay _balllauncherfirerate)
    (goto _label Open)
    (else
      (Utilities|FlowControl|Gate true :!label _label
        (:Exit
          (bind _lookdirection (Default|GetPlayerLookDir (Variables|Default|GetPlayerRef)))
          (Game|SpawnActorfromClass "/Game/Blueprints/BP_ProjectileBall.BP_ProjectileBall_C" (Math|Transform|MakeTransform (+ (* _lookdirection 2.0) (.location _returnvalue)) (.rotation _returnvalue) (.scale _returnvalue)) "Undefined" "MultiplyWithRoot" 0 0)
          (goto _label Close))))))

(event Input|EnhancedActionEvents|EnhancedInputActionIA_Primary
  (params (ActionValue :type Boolean) (ElapsedSeconds :type Float%20%28double-precision%29) (TriggeredSeconds :type Float%20%28double-precision%29) (InputAction :type Input%20Action%20Object%20Reference :default "/Game/Inputs/InputActions/IA_Primary.IA_Primary"))
  (bind _playerref (Variables|Default|GetPlayerRef))
  (bind _camera (Variables|/Game/Blueprints/BP_PlayerCharacter.BP_PlayerCharacter_C|GetCamera _playerref))
  (bind _returnvalue (Transformation|GetWorldTransform _camera))
  ;[1 1 1] Ball Launcher
  (:Triggered
    (Utilities|FlowControl|Gate true :!label _label
      (:Exit
        (bind _lookdirection (Default|GetPlayerLookDir (Variables|Default|GetPlayerRef)))
        (Game|SpawnActorfromClass "/Game/Blueprints/BP_ProjectileBall.BP_ProjectileBall_C" (Math|Transform|MakeTransform (+ (* _lookdirection 2.0) (.location _returnvalue)) (.rotation _returnvalue) (.scale _returnvalue)) "Undefined" "MultiplyWithRoot" 0 0)
        (goto _label Close))))
  (:Completed
    (goto _label Open)))

(event EventBeginPlay
  ;[1 1 1] Ball Launcher
  (bind _asbp_player_character (Utilities|Casting|CastToBP_PlayerCharacter (Components|GetOwner)))
  (Variables|Default|SetPlayerRef _asbp_player_character))