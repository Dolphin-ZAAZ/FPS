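; Player component that turns a held jump into a jetpack limited by the Energy vital.
; While IA_Jump triggers, it drains energy from CPlayerVitals and, if any remains, sets a very long JumpMaxHoldTime to sustain the Jump.
; Releasing the input or running out zeroes the hold time and stops the jump.
; The locally controlled character binds its landed delegate on BeginPlay to refill energy.
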(event Custom|ResetEnergy
  (params (Hit :type Hit%20Result%20Structure%20%28by%20ref%29))
  (Default|AddEnergy (Variables|/Game/Blueprints/Player/BP_PlayerCharacter.BP_PlayerCharacter_C|GetC_PlayerVitals (Variables|Default|GetPlayerRef)) 1e+06))

(event Input|EnhancedActionEvents|EnhancedInputActionIA_Jump
  (params (ActionValue :type Boolean) (ElapsedSeconds :type Float%20%28double-precision%29) (TriggeredSeconds :type Float%20%28double-precision%29) (InputAction :type Input%20Action%20Object%20Reference :default "/Game/Inputs/InputActions/Player/IA_Jump.IA_Jump"))
  (bind _playerref (Variables|Default|GetPlayerRef))
  (bind _c_playervitals (Variables|/Game/Blueprints/Player/BP_PlayerCharacter.BP_PlayerCharacter_C|GetC_PlayerVitals _playerref))
  (:Triggered
    (Default|RemoveEnergy _c_playervitals)
    (bind _energy (Default|GetVitals _c_playervitals))
    (if (> _energy 0.0)
      (Variables|/Script/Engine.Character|SetJumpMaxHoldTime _playerref 1e+03)
      (Character|Jump _playerref)
      (else
        (Variables|/Script/Engine.Character|SetJumpMaxHoldTime _playerref 0.0)
        (Character|StopJumping _playerref))))
  (:Completed
    (Variables|/Script/Engine.Character|SetJumpMaxHoldTime _playerref 0.0)
    (Character|StopJumping _playerref)))

(event EventBeginPlay
  (bind _asbp_player_character (Utilities|Casting|CastToBP_PlayerCharacter (Components|GetOwner)))
  (if (Pawn|IsLocallyControlled _asbp_player_character)
    (bind _output_get (Variables|Default|SetPlayerRef _asbp_player_character))
    (EventDispatchers|AssignLandedDelegate _output_get (delegate Custom|ResetEnergy))))