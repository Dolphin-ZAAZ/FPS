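; Player component that handles grid-based block building: previewing, placing and removing BP_Block actors.
; An input toggle flips build mode, during which Tick moves a collision-free preview block to the player's raycast target.
; Positions snap to a 100-unit grid after a nudge along the hit normal; preview and placement only work with UseGrid on.
; Secondary input places blocks, Interact destroys the targeted one, and both fire BlockPlaced.
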(event Input|EnhancedActionEvents|EnhancedInputActionIA_BuildModeToggle
  (params (ActionValue :type Boolean) (ElapsedSeconds :type Float%20%28double-precision%29) (TriggeredSeconds :type Float%20%28double-precision%29) (InputAction :type Input%20Action%20Object%20Reference :default "/Game/Inputs/InputActions/Player/IA_BuildModeToggle.IA_BuildModeToggle"))
  (:Started
    (Utilities|FlowControl|FlipFlop
      (:A
        (Variables|Default|SetBuildModeActive true))
      (:B
        (Variables|Default|SetBuildModeActive false)))
    (Default|CheckBuildMode (Variables|/Game/Blueprints/Player/BP_PlayerCharacter.BP_PlayerCharacter_C|GetHUD (Variables|Default|GetPlayerReference)))))

(event Input|EnhancedActionEvents|EnhancedInputActionIA_Interact
  (params (ActionValue :type Boolean) (ElapsedSeconds :type Float%20%28double-precision%29) (TriggeredSeconds :type Float%20%28double-precision%29) (InputAction :type Input%20Action%20Object%20Reference :default "/Game/Inputs/InputActions/Player/IA_Interact.IA_Interact"))
  (:Started
    (if (Variables|Default|GetBuildModeActive)
      (CallFunction|PickUpBlock)
      (Default|CallBlockPlaced))))

(event Input|EnhancedActionEvents|EnhancedInputActionIA_Secondary
  (params (ActionValue :type Boolean) (ElapsedSeconds :type Float%20%28double-precision%29) (TriggeredSeconds :type Float%20%28double-precision%29) (InputAction :type Input%20Action%20Object%20Reference :default "/Game/Inputs/InputActions/Player/IA_Secondary.IA_Secondary"))
  (:Started
    (if (Variables|Default|GetBuildModeActive)
      (CallFunction|PlaceBlock)
      (Default|CallBlockPlaced))))

(event EventBeginPlay
  (bind _asbp_player_character (Utilities|Casting|CastToBP_PlayerCharacter (Components|GetOwner))
    (:then
      (Variables|Default|SetPlayerReference _asbp_player_character))
    (:CastFailed
      (Development|PrintString "Block Placement Component active on a non-player-character"))))

(event EventTick
  (params (DeltaSeconds :type Float%20%28single-precision%29))
  (bind _previewblock (Variables|Default|GetPreviewBlock))
  (if (Variables|Default|GetBuildModeActive)
    (CallFunction|PreviewPlacement)
    (elif (Utilities|IsValid _previewblock)
      (Actor|DestroyActor _previewblock))))

(fn PlaceBlock
  (bind _rayhit (Default|PlayerRaycast (Variables|Default|GetPlayerReference)))
  (bind _output_get (Variables|Default|SetLookPoint (.ImpactPoint (Collision|BreakHitResult _rayhit))))
  (if (Variables|Default|GetUseGrid)
    (bind _output_get_2 (Variables|Default|SetGridPoint (Math|Vector|MakeVector (Math|Conversions|ToFloat(Integer) (* (Math|Float|Round (/ (+ (Math|Float|Round (.x _output_get)) (.x (.Normal (Collision|BreakHitResult _rayhit)))) 100)) 100)) (Math|Conversions|ToFloat(Integer) (* (Math|Float|Round (/ (+ (Math|Float|Round (.y _output_get)) (.y (.Normal (Collision|BreakHitResult _rayhit)))) 100)) 100)) (Math|Conversions|ToFloat(Integer) (* (Math|Float|Round (/ (+ (Math|Float|Round (.z _output_get)) (.z (.Normal (Collision|BreakHitResult _rayhit)))) 100)) 100)))))
    (if (Utilities|Operators|NotEqual(!=) :A (Variables|Default|GetLookPoint))
      (bind _returnvalue (Game|SpawnActorfromClass "/Game/Blueprints/Items/BP_Block.BP_Block_C" (Math|Conversions|ToTransform(Vector) (Variables|Default|GetLookPoint)) "Undefined" "MultiplyWithRoot" 0 0))
      (Transformation|SetActorLocation _returnvalue _output_get_2 false false))))

(fn PickUpBlock
  (bind _rayhit (Default|PlayerRaycast (Variables|Default|GetPlayerReference)))
  (Utilities|Casting|CastToBP_BlockClass (Utilities|GetClass (.HitActor (Collision|BreakHitResult _rayhit))))
  (if true
    (Actor|DestroyActor (.HitActor (Collision|BreakHitResult _rayhit)))))

(fn PreviewPlacement
  (bind _rayhit (Default|PlayerRaycast (Variables|Default|GetPlayerReference)))
  (bind _output_get (Variables|Default|SetLookPoint (.ImpactPoint (Collision|BreakHitResult _rayhit))))
  (if (Variables|Default|GetUseGrid)
    (bind _output_get_2 (Variables|Default|SetGridPoint (Math|Vector|MakeVector (Math|Conversions|ToFloat(Integer) (* (Math|Float|Round (/ (+ (Math|Float|Round (.x _output_get)) (.x (.Normal (Collision|BreakHitResult _rayhit)))) 100)) 100)) (Math|Conversions|ToFloat(Integer) (* (Math|Float|Round (/ (+ (Math|Float|Round (.y _output_get)) (.y (.Normal (Collision|BreakHitResult _rayhit)))) 100)) 100)) (Math|Conversions|ToFloat(Integer) (* (Math|Float|Round (/ (+ (Math|Float|Round (.z _output_get)) (.z (.Normal (Collision|BreakHitResult _rayhit)))) 100)) 100)))))
    (if (Utilities|Operators|NotEqual(!=) :A (Variables|Default|GetLookPoint))
      (if (Utilities|IsValid (Variables|Default|GetPreviewBlock))
        (bind _asbp_block (Utilities|Casting|CastToBP_Block (.HitActor (Collision|BreakHitResult _rayhit)) :!label _label)
          (:then
            (if (not (== _asbp_block (Variables|Default|GetPreviewBlock)))
              (Transformation|SetActorLocation (stale _output_get_3) _output_get_2 false false :!label _label_2)))
          (:CastFailed
            (goto _label_2)))
        (else
          (bind _returnvalue (Game|SpawnActorfromClass "/Game/Blueprints/Items/BP_Block.BP_Block_C" (Math|Conversions|ToTransform(Vector) (Variables|Default|GetLookPoint)) "Undefined" "MultiplyWithRoot" 0 0))
          (bind _output_get_3 (Variables|Default|SetPreviewBlock _returnvalue))
          (Collision|SetCollisionEnabled (Variables|/Game/Blueprints/Items/BP_Block.BP_Block_C|GetCube _output_get_3) "NoCollision")
          (if (Utilities|IsValid (Variables|Default|GetPreviewBlock))
            (goto _label)))))))