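; Player component that controls the inventory screen, creating the UI_Inventory widget and adding or removing it from the viewport.
; The toggle input opens it on trigger (through a FlipFlop with only A wired) and closes it on completion unless locked.
; The lock input keeps it open with the mouse cursor shown until toggled again.
; Transitions set BP_PlayerCharacter's input state, and closing restores game-only input and mouse capture.
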(event Input|EnhancedActionEvents|EnhancedInputActionIA_LockInventory
  (params (ActionValue :type Boolean) (ElapsedSeconds :type Float%20%28double-precision%29) (TriggeredSeconds :type Float%20%28double-precision%29) (InputAction :type Input%20Action%20Object%20Reference :default "/Game/Inputs/InputActions/Inventory/IA_LockInventory.IA_LockInventory"))
  ;[1 1 1] Inventory GUI Controls
  (bind _inventory_open (CallFunction|GetInventoryOpen))
  (if _inventory_open
    (bind _inventorylocked (CallFunction|GetInventoryLocked))
    (if (not _inventorylocked)
      (CallFunction|LockInventory)
      (Default|SetInputState (Variables|Default|GetPlayerRef) "NewEnumerator2"))))

(event Input|EnhancedActionEvents|EnhancedInputActionIA_ToggleInventory
  (params (ActionValue :type Boolean) (ElapsedSeconds :type Float%20%28double-precision%29) (TriggeredSeconds :type Float%20%28double-precision%29) (InputAction :type Input%20Action%20Object%20Reference :default "/Game/Inputs/InputActions/Inventory/IA_ToggleInventory.IA_ToggleInventory"))
  (bind _playerref (Variables|Default|GetPlayerRef))
  ;[1 1 1] Inventory GUI Controls
  (:Triggered
    (Utilities|FlowControl|FlipFlop
      (:A
        (bind _inventorylocked (CallFunction|GetInventoryLocked))
        (if _inventorylocked
          (CallFunction|CloseInventory :!label _label)
          (Default|SetInputState _playerref "NewEnumerator0")
          (Class|WidgetBlueprintLibrary|SetFocustoGameViewport)
          (Class|GameplayStatics|SetViewportMouseCaptureMode "CapturePermanently")
          (else
            (bind _inventory_open (CallFunction|GetInventoryOpen))
            (if (not _inventory_open)
              (CallFunction|OpenInventory)
              (Default|SetInputState _playerref "NewEnumerator1")))))))
  (:Completed
    (bind _inventory_open_2 (CallFunction|GetInventoryOpen))
    (if _inventory_open_2
      (bind _inventorylocked_2 (CallFunction|GetInventoryLocked))
      (if (not _inventorylocked_2)
        (goto _label)))))

(event EventBeginPlay
  ;[1 1 1] Inventory GUI Controls
  (CallFunction|ConstructInventoryUI)
  (bind _asbp_player_character (Utilities|Casting|CastToBP_PlayerCharacter (Components|GetOwner)))
  (Variables|Default|SetPlayerRef _asbp_player_character)
  (CallFunction|OpenInventory)
  (CallFunction|CloseInventory))

(fn OpenInventory
  (UserInterface|Viewport|AddtoViewport (Variables|Default|GetInventoryUI) 0)
  (Variables|Default|SetInventoryOpen true))

(fn CloseInventory
  (bind _returnvalue (Game|GetPlayerCharacter 0))
  (bind _playerstate (Variables|/Script/Engine.Pawn|GetPlayerState _returnvalue))
  (bind _returnvalue_2 (Game|GetPlayerController _playerstate))
  (Widget|RemovefromParent (Variables|Default|GetInventoryUI))
  (Variables|/Script/Engine.PlayerController|SetbShowMouseCursor _returnvalue_2 false)
  (Variables|Default|SetInventoryOpen false)
  (Variables|Default|SetInventoryLocked false)
  (Input|SetInputModeGameOnly _returnvalue_2 false))

(fn LockInventory
  (Variables|/Script/Engine.PlayerController|SetbShowMouseCursor (Game|GetPlayerController (Variables|/Script/Engine.Pawn|GetPlayerState (Game|GetPlayerCharacter 0))) true)
  (Variables|Default|SetInventoryLocked true))

(fn GetInventoryOpen
  (return (Variables|Default|GetInventoryOpen)))

(fn GetInventoryLocked
  (return (Variables|Default|GetInventoryLocked)))

(fn ConstructInventoryUI
  (bind _returnvalue (UserInterface|CreateWidget "/Game/Blueprints/UI/UI_Inventory.UI_Inventory_C" (Game|GetPlayerController 0)))
  (Variables|Default|SetInventoryUI _returnvalue))