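; Base Blueprint for items in the player inventory system, defining the shared equip, use, drop, favourite and delete functions.
; Equip stops physics on the hitbox, applies EquipTransform to the root as a relative transform and flags the item equipped.
; DeleteItem calls a server RPC on player 0's inventory component, then hides the item.
; Favourite, Use, Drop and UseEffects are empty stubs.
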(fn ConstructionScript)

(fn Favourite)

(fn Equip
  (params (OwningPlayer :type Boolean))
  (Physics|SetSimulatePhysics (Variables|Default|GetHitbox) false)
  (Transformation|SetRelativeTransform (Variables|Default|GetDefaultSceneRoot) (Variables|Default|GetEquipTransform) false false)
  (Variables|Default|SetIsEquipped true))

(fn Use
  (params (PlayerRef :type BP%20Player%20Character%20Object%20Reference) (IsInstigator :type Boolean)))

(fn Drop)

(fn DeleteItem
  (bind _defaultsceneroot (Variables|Default|GetDefaultSceneRoot))
  (bind _asbp_player_character (Utilities|Casting|CastToBP_PlayerCharacter (Game|GetPlayerCharacter 0)))
  (Default|ServerRPCDeleteItem (Variables|/Game/Blueprints/Player/BP_PlayerCharacter.BP_PlayerCharacter_C|GetC_PlayerInventory _asbp_player_character) self)
  (Utilities|IsValid _defaultsceneroot
    (:Is%20Valid
      (Rendering|SetVisibility _defaultsceneroot false true))))

(fn UseEffects
  (params (Location :type Vector)))