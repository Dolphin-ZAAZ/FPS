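; BP_PhysicsBlock is a block actor that joins itself to adjacent physics blocks with breakable physics constraints.
; On BeginPlay, it line-traces along six world axes, creates a constraint to each block found, then calls RefreshJoints on those neighbours.
; RefreshJoints re-traces and may add constraints when joints number fewer than trace results.
; Each joint gets locked angular limits and a break threshold scaled from AngularThreshold.
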(event EventBeginPlay
  (CallFunction|CreateInitialJoints))

(fn ConstructionScript)

(fn CreateInitialJoints
  (bind _staticmeshcomponent (Variables|Default|GetStaticMeshComponent))
  (bind _staticmeshcomponent_2 (Variables|Default|GetStaticMeshComponent))
  (bind _returnvalue (Transformation|GetWorldLocation _staticmeshcomponent_2))
  (bind _returnvalue_2 (Transformation|GetWorldLocation _staticmeshcomponent))
  (Utilities|Array|Add (Variables|Default|GetCube%20Axis) (+ _returnvalue "100.000000,0.000000,0.000000"))
  (Utilities|Array|Add (Variables|Default|GetCube%20Axis) (+ _returnvalue "0.000000,100.000000,0.000000"))
  (Utilities|Array|Add (Variables|Default|GetCube%20Axis) (+ _returnvalue "0.000000,0.000000,100.000000"))
  (Utilities|Array|Add (Variables|Default|GetCube%20Axis) (+ _returnvalue "-100.000000,0.000000,0.000000"))
  (Utilities|Array|Add (Variables|Default|GetCube%20Axis) (+ _returnvalue "0.000000,-100.000000,0.000000"))
  (Utilities|Array|Add (Variables|Default|GetCube%20Axis) (+ _returnvalue "0.000000,0.000000,-100.000000"))
  (for _array_element (Variables|Default|GetCube%20Axis)
    (bind _outhit (Collision|LineTraceForObjects (Math|Vector|MakeVector (.x _returnvalue_2) (.y _returnvalue_2) (+ (.z _returnvalue_2) 5e+01)) (Math|Vector|MakeVector (.x _array_element) (.y _array_element) (+ (.z _array_element) 5e+01)) (Variables|Default|GetObject%20Types) false 0 "None"))
    (Utilities|Array|Add (Variables|Default|GetAdjacentObjects) (.hitactor _outhit)))
  (for _array_element_2 (Variables|Default|GetAdjacentObjects)
    (bind _asbp_physics_block (Utilities|Casting|CastToBP_PhysicsBlock _array_element_2))
    (bind _returnvalue_3 (AddComponent|AddPhysicsConstraintComponent false))
    (Utilities|Array|Add (Variables|Default|GetJoints) _returnvalue_3)
    (Class|PhysicsConstraintComponent|SetConstrainedComponents _returnvalue_3 (Variables|Default|GetStaticMeshComponent) "None" (Variables|/Script/Engine.StaticMeshActor|GetStaticMeshComponent _asbp_physics_block) "None"))
  (for _array_element_3 (Variables|Default|GetJoints)
    (CallFunction|SetJointParameters _array_element_3))
  (for _array_element_4 (Variables|Default|GetAdjacentObjects)
    (bind _asbp_physics_block_2 (Utilities|Casting|CastToBP_PhysicsBlock _array_element_4))
    (CallFunction|RefreshJoints _asbp_physics_block_2)))

(fn RefreshJoints
  (Utilities|Array|Clear (Variables|Default|GetAdjacentObjects))
  (for _array_element (Variables|Default|GetCube%20Axis)
    (bind _outhit (Collision|LineTraceForObjects (Transformation|GetWorldLocation (Variables|Default|GetStaticMeshComponent)) _array_element (Variables|Default|GetObject%20Types) false 0 "None"))
    (Utilities|Array|Add (Variables|Default|GetAdjacentObjects) (.hitactor _outhit)))
  (if (< (Utilities|Array|Length (Variables|Default|GetJoints)) (Utilities|Array|Length (Variables|Default|GetAdjacentObjects)))
    (for _array_element_2 (Variables|Default|GetAdjacentObjects)
      (bind _asbp_physics_block (Utilities|Casting|CastToBP_PhysicsBlock _array_element_2))
      (bind _array_element_3 (Utilities|Array|ForEachLoopwithBreak (Variables|Default|GetJoints) :!label _label)
        (:LoopBody
          (bind _outcomponent2 (Class|PhysicsConstraintComponent|GetConstrainedComponents _array_element_3))
          (if (== _outcomponent2 (Variables|/Script/Engine.StaticMeshActor|GetStaticMeshComponent _asbp_physics_block))
            (goto _label Break)
            (else
              (bind _returnvalue (AddComponent|AddPhysicsConstraintComponent false))
              (Class|PhysicsConstraintComponent|SetConstrainedComponents _returnvalue (Variables|Default|GetStaticMeshComponent) "None" (Variables|/Script/Engine.StaticMeshActor|GetStaticMeshComponent _asbp_physics_block) "None")
              (Utilities|Array|Add (Variables|Default|GetJoints) _returnvalue))))))
    (for _array_element_4 (Variables|Default|GetJoints)
      (CallFunction|SetJointParameters _array_element_4))))

(fn SetJointParameters
  (params (self2 :type Physics%20Constraint%20Component%20Object%20Reference))
  (bind _returnvalue (Class|PhysicsConstraintComponent|GetConstraint self2))
  (Class|ConstraintInstanceBlueprintLibrary|SetAngularBreakable _returnvalue true (* (Variables|Default|GetAngularThreshold) 1e+10))
  (Class|ConstraintInstanceBlueprintLibrary|SetAngularLimits _returnvalue "ACM_Locked" 0.0 "ACM_Locked" 0.0 "ACM_Locked" 0.0))