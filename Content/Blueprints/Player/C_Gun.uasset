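; C_Gun is the player's hitscan gun component, caching the owning BP_PlayerCharacter and deriving a fire interval from rounds per minute for local control.
; IA_Primary waits that interval through a Delay before raycasting from the player, optionally spawning BP_Explosion at the impact point, even without a blocking hit.
; Player-damageable I_Damageable targets lose health, multiplied on components named "CritSpot", and receive a touch perception event.
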(event Input|EnhancedActionEvents|EnhancedInputActionIA_Primary
  (params (ActionValue :type Boolean) (ElapsedSeconds :type Float%20%28double-precision%29) (TriggeredSeconds :type Float%20%28double-precision%29) (InputAction :type Input%20Action%20Object%20Reference :default "/Game/Inputs/InputActions/Player/IA_Primary.IA_Primary"))
  (bind _damage (Variables|Default|GetDamage))
  (Utilities|FlowControl|Delay (Variables|Default|GetFireInterval))
  (bind _rayhit (Default|PlayerRaycast (Variables|Default|GetPlayerRef)))
  (if (Variables|Default|GetHasExplosiveBullets)
    (Game|SpawnActorfromClass "/Game/Blueprints/Player/BP_Explosion.BP_Explosion_C" (Math|Conversions|ToTransform(Vector) (.ImpactPoint (Collision|BreakHitResult _rayhit))) "Undefined" "MultiplyWithRoot" 0 0))
  (if (.bBlockingHit (Collision|BreakHitResult _rayhit))
    (bind _asi_damageable (Utilities|Casting|CastToI_Damageable (.HitActor (Collision|BreakHitResult _rayhit))))
    (bind _playerdamageable (Default|PlayerDamageable _asi_damageable))
    (if _playerdamageable
      (if (Utilities|Enum|Equal(Enum) (Utilities|GetObjectName (.HitComponent (Collision|BreakHitResult _rayhit))) "CritSpot")
        (Default|RemoveHealth _asi_damageable (* (Variables|Default|GetCritMultiplier) _damage))
        (else
          (Default|RemoveHealth _asi_damageable _damage)))
      (Class|AISenseTouch|ReportTouchEvent (.HitActor (Collision|BreakHitResult _rayhit)) (Variables|Default|GetPlayerRef) (.ImpactPoint (Collision|BreakHitResult _rayhit))))))

(event EventBeginPlay
  (bind _returnvalue (Components|GetOwner))
  (if (Pawn|IsLocallyControlled (Variables|/Script/Engine.Actor|GetInstigator _returnvalue))
    (bind _asbp_player_character (Utilities|Casting|CastToBP_PlayerCharacter _returnvalue))
    (Variables|Default|SetPlayerRef _asbp_player_character)
    (Variables|Default|SetFireInterval (/ 1.0 (/ (Variables|Default|GetRoundsPerMinute) 6e+01)))))