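; Player vitals component that tracks health and energy, broadcasts their changes, and handles death and respawn.
; Additions clamp to maximums from the owner's player stats component, while energy drains one point at a time.
; Zero health shows the death screen with UI-only input and sets a dead flag on the game instance singleton.
; Respawn teleports to a hardcoded location, restores game input and refills health only.
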(event EventBeginPlay
  (bind _returnvalue (Components|GetOwner))
  (if (Pawn|IsLocallyControlled (Variables|/Script/Engine.Actor|GetInstigator _returnvalue))
    (bind _asbp_player_character (Utilities|Casting|CastToBP_PlayerCharacter _returnvalue))
    (Variables|Default|SetPlayerRef _asbp_player_character)))

(fn RemoveHealth
  (params (HealthAmount :type Float%20%28double-precision%29))
  (bind _output_get (Variables|Default|SetHealth (- (Variables|Default|GetHealth) HealthAmount)))
  (Default|CallHealthChanged)
  (if (<= _output_get 0.0)
    (CallFunction|KillPlayer)))

(fn AddHealth
  (params (HealthAmount :type Float%20%28double-precision%29))
  (bind _playerstats (CallFunction|GetStats))
  (if (> (+ HealthAmount (Variables|Default|GetHealth)) (.maxhealth _playerstats))
    (Variables|Default|SetHealth (.maxhealth _playerstats))
    (else
      (Variables|Default|SetHealth (+ HealthAmount (Variables|Default|GetHealth)))))
  (Default|CallHealthChanged))

(fn RemoveEnergy
  (if (>= (- (Variables|Default|GetEnergy) 1.0) 0.0)
    (Variables|Default|SetEnergy (- (Variables|Default|GetEnergy) 1.0))
    (Default|CallEnergyChanged)))

(fn AddEnergy
  (params (EnergyAmount :type Float%20%28double-precision%29))
  (bind _playerstats (CallFunction|GetStats))
  (if (> (+ (Variables|Default|GetEnergy) EnergyAmount) (.maxenergy _playerstats))
    (Variables|Default|SetEnergy (.maxenergy _playerstats))
    (else
      (Variables|Default|SetEnergy (+ (Variables|Default|GetEnergy) EnergyAmount))))
  (Default|CallEnergyChanged))

(fn Exhausted)

(fn KillPlayer
  (bind _returnvalue (Game|GetPlayerController 0))
  (bind _asbp_global_singleton (Utilities|Casting|CastToBP_GlobalSingleton (Game|GetGameInstance)))
  (bind _playerisdead (Default|GetPlayerIsDead _asbp_global_singleton))
  (if (not _playerisdead)
    (bind _returnvalue_2 (UserInterface|CreateWidget "/Game/Blueprints/Player/UI/UI_DeathScreen.UI_DeathScreen_C" _returnvalue))
    (bind _output_get (Variables|Default|SetDeathScreen _returnvalue_2))
    (UserInterface|Viewport|AddtoViewport _output_get 0)
    (Variables|/Script/Engine.PlayerController|SetbShowMouseCursor _returnvalue true)
    (Input|SetInputModeUIOnly _returnvalue 0 "DoNotLock" false)
    (bind _asbp_global_singleton_2 (Utilities|Casting|CastToBP_GlobalSingleton (Game|GetGameInstance)))
    (Default|SetPlayerIsDead _asbp_global_singleton_2 true)
    (Default|CallPlayerDied)))

(fn GetStats
  (bind _asbp_player_character (Utilities|Casting|CastToBP_PlayerCharacter (Components|GetOwner)))
  (return (Variables|/Game/Blueprints/Player/C_PlayerStats.C_PlayerStats_C|GetStats (Variables|/Game/Blueprints/Player/BP_PlayerCharacter.BP_PlayerCharacter_C|GetC_PlayerStats _asbp_player_character))))

(fn Respawn
  (bind _returnvalue (Game|GetPlayerController 0))
  (Widget|RemovefromParent (Variables|Default|GetDeathScreen))
  (Transformation|SetActorLocation (Components|GetOwner) "-510.000000,0.000000,100.000000" false false)
  (Input|SetInputModeGameOnly _returnvalue false)
  (Variables|/Script/Engine.PlayerController|SetbShowMouseCursor _returnvalue false)
  (bind _playerstats (CallFunction|GetStats))
  (Variables|Default|SetHealth (.maxhealth _playerstats))
  (Default|CallHealthChanged))

(fn GetVitals
  (return (Variables|Default|GetHealth) (Variables|Default|GetEnergy)))